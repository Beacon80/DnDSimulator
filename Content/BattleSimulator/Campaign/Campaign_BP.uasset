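; Campaign Blueprint for the battle simulator that supplies its available characters to the gameplay game mode.
; LoadCharacterListEvent fetches GameplayGM through the GameplayRef cast helper and passes AvailableCharacters to FillAvailableCharacterListEvent.
; LCLE is a debug event that prints differently on server and client.
; Leftover unconnected nodes call LCLE and run a LobbyPC player-controller check, but never execute.
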(event Custom|LCLE
  (if (Networking|IsServer)
    (Development|PrintString "Ping")
    (else
      (Development|PrintString "Pong"))))

(event EventLoadCharacterListEvent
  (bind _asgameplay_gm (Utilities|GameplayRef))
  (Default|FillAvailableCharacterListEvent _asgameplay_gm (Variables|Default|GetavailableCharacters)))

(fn ConstructionScript)