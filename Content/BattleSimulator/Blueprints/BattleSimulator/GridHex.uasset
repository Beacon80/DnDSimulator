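; GridHex is a hex tile actor for the battle simulator grid that shows a highlight on its Cylinder component.
; SetHighlightBP switches on the highlight state, enabling custom depth rendering for states 1 and 2 and disabling it otherwise.
; Both highlighted states render identically, as the stencil value and visibility nodes that might distinguish them are disconnected.
; The Cylinder release event is empty, and the construction script only calls its parent.
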(event OnReleased(Cylinder)
  (params (TouchedComponent :type Primitive%20Component%20Object%20Reference) (ButtonReleased :type Key%20Structure)))

(event EventBeginPlay
  (|CallParentFunction) ; This node is disabled and will not be called.\nDrag off pins to build functionality.
)

(event Collision|EventActorBeginOverlap
  (params (OtherActor :type Actor%20Object%20Reference))
  (|CallParentFunction OtherActor) ; This node is disabled and will not be called.\nDrag off pins to build functionality.
)

(event EventTick
  (params (DeltaSeconds :type Float%20%28single-precision%29))
  (|CallParentFunction DeltaSeconds) ; This node is disabled and will not be called.\nDrag off pins to build functionality.
)

(event EventSetHighlightBP
  (params (gh :type Integer))
  (bind _cylinder (Variables|Default|GetCylinder))
  (switch int gh
    (:Default
      (Rendering|SetRenderCustomDepth _cylinder false :!label _label))
    (:0
      (goto _label))
    (:1
      (Rendering|SetRenderCustomDepth _cylinder true))
    (:2
      (Rendering|SetRenderCustomDepth _cylinder true))))

(fn ConstructionScript
  (|CallParentFunction))