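; Grid square actor for the battle simulator that shows a highlight state on its cube mesh.
; The SetHighlightBP event switches on the highlight value, turning custom depth rendering off for the first state and on for the other three, which therefore render alike.
; Disconnected nodes for per-state cube scaling (none, selected, adjacent, corner) remain unused, and the cylinder's release event is empty.
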(event OnReleased(Cylinder)
  (params (TouchedComponent :type Primitive%20Component%20Object%20Reference) (ButtonReleased :type Key%20Structure :default "None")))

(event EventBeginPlay
  (|CallParentFunction) ; This node is disabled and will not be called.\nDrag off pins to build functionality.
)

(event Collision|EventActorBeginOverlap
  (params (OtherActor :type Actor%20Object%20Reference))
  (|CallParentFunction OtherActor) ; This node is disabled and will not be called.\nDrag off pins to build functionality.
)

(event EventTick
  (params (DeltaSeconds :type Float%20%28single-precision%29))
  (|CallParentFunction DeltaSeconds) ; This node is disabled and will not be called.\nDrag off pins to build functionality.
)

(event EventSetHighlightBP
  (params (gh :type Integer))
  (bind _cube (Variables|Default|GetCube))
  (switch int gh
    (:0
      (Rendering|SetRenderCustomDepth _cube false))
    (:1
      (Rendering|SetRenderCustomDepth _cube true))
    (:2
      (Rendering|SetRenderCustomDepth _cube true))
    (:3
      (Rendering|SetRenderCustomDepth _cube true))))

(fn ConstructionScript
  (|CallParentFunction))