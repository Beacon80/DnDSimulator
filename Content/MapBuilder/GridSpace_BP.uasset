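; Grid space actor for the map builder, representing one space that can be clicked and selected.
; On release, it passes itself to MapBuilderController_BP through GridClick and then SelectSpace.
; MoveCameratoSpace shifts the view by setting the TopDownCharacter's location to the space's own location, without sweeping.
; Controller and character references are looked up by class on first use and cached while valid.
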(event EventActorOnReleased
  (params (ButtonReleased :type Key%20Structure :default "None"))
  (bind _newparam (CallFunction|GetMapBuilderController))
  (Class|MapBuilderController|GridClick _newparam self)
  (Default|SelectSpace _newparam self))

(event EventMoveCameratoSpace
  (CallFunction|SetCameraLocationtoGrid))

(fn ConstructionScript)

(fn SetCameraLocationtoGrid
  (bind _retcharacterptr (CallFunction|GetCharacterPtr))
  (Transformation|SetActorLocation _retcharacterptr (Transformation|GetActorLocation) false false))

(fn GetCharacterPtr
  (Utilities|IsValid (Variables|Default|GetcharacterPtr)
    (:Is%20Valid
      _)
    (:Is%20Not%20Valid
      (bind _returnvalue (Actor|GetActorOfClass "/Game/TopDownBP/Blueprints/TopDownCharacter.TopDownCharacter_C"))
      (bind _output_get (Variables|Default|SetcharacterPtr _returnvalue))))
  (return _output_get))

(fn GetMapBuilderController
  (Utilities|IsValid (Variables|Default|GetmapBuilderController)
    (:Is%20Valid
      _)
    (:Is%20Not%20Valid
      (bind _returnvalue (Actor|GetActorOfClass "/Game/MapBuilder/MapBuilderController_BP.MapBuilderController_BP_C"))
      (bind _output_get (Variables|Default|SetmapBuilderController _returnvalue))))
  (return _output_get))