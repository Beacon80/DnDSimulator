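; Player controller for the map builder that tracks the selected space and handles movement and camera-centering input.
; Move axes feed movement input to a TopDownCharacter, though both pass a zero world direction.
; SelectSpace stores the space and updates the MapBuilderUI, and the CenterOnSpace action moves the camera to that space's grid location.
; Character and UI references are found by class on first use and cached.
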(event EventBeginPlay)

(event Collision|EventActorBeginOverlap
  (params (OtherActor :type Actor%20Object%20Reference)))

(event EventTick
  (params (DeltaSeconds :type Float%20%28single-precision%29)))

(event Input|ActionEvents|InputActionCenterOnSpace
  (params (Key :type Key%20Structure :default "None"))
  (bind _selectedspace (Variables|Default|GetselectedSpace))
  (:Released
    (Utilities|IsValid _selectedspace
      (:Is%20Valid
        (Default|SetCameraLocationtoGrid _selectedspace)))))

(event Input|AxisEvents|InputAxisMoveForward
  (params (AxisValue :type Float%20%28single-precision%29))
  (bind _retcharacterptr (CallFunction|GetCharacterPtr))
  (Pawn|Input|AddMovementInput _retcharacterptr "0, 0, 0" AxisValue false))

(event Input|AxisEvents|InputAxisMoveRight
  (params (AxisValue :type Float%20%28single-precision%29))
  (bind _retcharacterptr (CallFunction|GetCharacterPtr))
  (Pawn|Input|AddMovementInput _retcharacterptr "0, 0, 0" AxisValue false))

(fn ConstructionScript)

(fn GetCharacterPtr
  (Utilities|IsValid (Variables|Default|GettopDownCharacter)
    (:Is%20Valid
      _)
    (:Is%20Not%20Valid
      (bind _returnvalue (Actor|GetActorOfClass "/Game/TopDownBP/Blueprints/TopDownCharacter.TopDownCharacter_C"))
      (bind _output_get (Variables|Default|SettopDownCharacter _returnvalue))))
  (return _output_get))

(fn SelectSpace
  (params (newSpace :type Grid%20Space%20BP%20Object%20Reference))
  (bind _output_get (Variables|Default|SetselectedSpace newSpace))
  (bind _retmbui (CallFunction|GetMBUI))
  (Default|UpdateSpace _retmbui _output_get))

(fn CenterCameraonSpace
  (bind _selectedspace (Variables|Default|GetselectedSpace))
  (Utilities|IsValid _selectedspace
    (:Is%20Valid
      (Default|SetCameraLocationtoGrid _selectedspace))))

(fn GetMBUI
  (Utilities|IsValid (Variables|Default|GetmapBuilderUI)
    (:Is%20Valid
      _)
    (:Is%20Not%20Valid
      (bind _foundwidgets (Widget|GetAllWidgetsOfClass "/Game/MapBuilder/MapBuilderUI.MapBuilderUI_C" true))
      (bind _output_get (Variables|Default|SetmapBuilderUI (Utilities|Array|Get(acopy) _foundwidgets)))))
  (return _output_get))